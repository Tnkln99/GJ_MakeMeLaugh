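; Game mode for a two-player local fighting match that sets up both players and ends the fight when one fighter dies.
; BeginPlay gives each player controller its own input mapping context, creating the second local player if missing, then runs each controller's Setup.
; It binds both fighters to a shared HUD and listens for their death.
; A death prints the winner, disables the loser's controller, and returns to the main menu after a short delay.
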(event `self.ReceiveBeginPlay`
  (bind _returnvalue (`GameplayStatics.GetPlayerController` 0))
  (bind _returnvalue_2 (`GameplayStatics.GetPlayerController` 1))
  (bind _returnvalue_3 (`GameplayStatics.GetPlayerController` 0))
  (bind _returnvalue_4 (`GameplayStatics.GetPlayerController` 0))
  (`|ExecutionSequence`
    (:`then_0`
      ;[1 1 1] Player Controller 1
      (`EnhancedInputSubsystemInterface.AddMappingContext` (pcsubsystem `EnhancedInputLocalPlayerSubsystem` _returnvalue_3) "/Game/Inputs/IMC_Fighter1.IMC_Fighter1" 0 (struct))
      (bind _asbp_controller (cast `/Game/Actors/BP_Controller` _returnvalue_3))
      (`/Game/Actors/BP_Controller.Setup` _asbp_controller 0))
    (:`then_1`
      ;[1 1 1] Player Controller 2
      (`/Engine/EditorBlueprintResources/StandardMacros.IsValid` _returnvalue_2
        (:`Is Valid`
          (`EnhancedInputSubsystemInterface.AddMappingContext` (pcsubsystem `EnhancedInputLocalPlayerSubsystem` _returnvalue_2) "/Game/Inputs/IMC_Fighter2.IMC_Fighter2" 0 (struct))
          (bind _asbp_controller_2 (cast `/Game/Actors/BP_Controller` _returnvalue_2))
          (`/Game/Actors/BP_Controller.Setup` _asbp_controller_2 1))
        (:`Is Not Valid`
          (bind _returnvalue_5 (`GameplayStatics.CreatePlayer` 1))
          (`EnhancedInputSubsystemInterface.AddMappingContext` (pcsubsystem `EnhancedInputLocalPlayerSubsystem` _returnvalue_5) "/Game/Inputs/IMC_Fighter2.IMC_Fighter2" 0 (struct))
          (bind _asbp_controller_3 (cast `/Game/Actors/BP_Controller` _returnvalue_5))
          (`/Game/Actors/BP_Controller.Setup` _asbp_controller_3 1))))
    (:`then_2`
      (bind _returnvalue_6 (`|CreateWidget` "/Game/Widget/WB_HUD.WB_HUD_C" _returnvalue_4))
      (`UserWidget.AddToViewport` _returnvalue_6 0)
      (bind _asbp_controller_4 (cast `/Game/Actors/BP_Controller` _returnvalue_4))
      (bind _fighter_ref (`/Game/Actors/BP_Controller.Fighter_Ref` _asbp_controller_4))
      (add `/Game/Actors/BP_Fighter.OnDie` _fighter_ref (delegate `Fighter1Dead`))
      (bind _asbp_controller_5 (cast `/Game/Actors/BP_Controller` (`GameplayStatics.GetPlayerController` 1)))
      (bind _fighter_ref_2 (`/Game/Actors/BP_Controller.Fighter_Ref` _asbp_controller_5))
      (add `/Game/Actors/BP_Fighter.OnDie` _fighter_ref_2 (delegate `Fighter2Deaed`))
      (`/Game/Widget/WB_HUD.BindFighters` _returnvalue_6 _fighter_ref _fighter_ref_2))
    (:`then_3`
      (`WidgetBlueprintLibrary.SetInputMode_GameOnly` _returnvalue)
      (`WidgetBlueprintLibrary.SetInputMode_GameOnly` (`GameplayStatics.GetPlayerController` 1))
      (set `PlayerController.bShowMouseCursor` false _returnvalue))))

(event `Fighter1Dead`
  (bind _returnvalue (`GameplayStatics.GetPlayerController` 0))
  (`KismetSystemLibrary.PrintString` "Fight Finished ! Fighter 2 wins !")
  (bind _asbp_controller (cast `/Game/Actors/BP_Controller` (`GameplayStatics.GetPlayerController` 0)))
  (set `/Game/Actors/BP_Controller.Disabled` true _asbp_controller)
  (`KismetSystemLibrary.Delay` 2.0 :!label _label)
  (`WidgetBlueprintLibrary.SetInputMode_UIOnlyEx` _returnvalue null)
  (`WidgetBlueprintLibrary.SetInputMode_UIOnlyEx` (`GameplayStatics.GetPlayerController` 1) null)
  (set `PlayerController.bShowMouseCursor` true _returnvalue)
  (`GameplayStatics.OpenLevelBySoftObjectPtr` "/Game/L_Menu/L_MainMenu.L_MainMenu"))

(event `Fighter2Deaed`
  (`KismetSystemLibrary.PrintString` "Fight Finished ! Fighter 1 wins !")
  (bind _asbp_controller (cast `/Game/Actors/BP_Controller` (`GameplayStatics.GetPlayerController` 1)))
  (set `/Game/Actors/BP_Controller.Disabled` true _asbp_controller)
  (goto _label))

(event `self.ReceiveTick`
  (params (DeltaSeconds :type "Float (single-precision)")))

(fn `UserConstructionScript`)