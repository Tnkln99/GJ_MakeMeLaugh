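; BP_Fighter is an indexed fighter actor with separate collision zones for head, upper body and lower body.
; Each zone's overlap event prints which fighter was hit and where; no damage logic is present.
; ApplyTiltRotation rolls the root Scene, yawed 180 degrees for fighter 1, and sets the mesh yaw from an input value.
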(event `self.HeadCollision.OnComponentBeginOverlap`
  (params (OverlappedComponent :type "PrimitiveComponent Object Reference") (OtherActor :type "Actor Object Reference") (OtherComp :type "PrimitiveComponent Object Reference") (OtherBodyIndex :type Integer) (bFromSweep :type Boolean) (SweepResult :type "HitResult Structure (by ref)"))
  (`KismetSystemLibrary.PrintText` (`|FormatText` "Fighter {Index} has been hit on the head !" (`self.FighterIndex`)) true true (struct :`R` 1.0 :`B` 0.237192 :`A` 1.0) 5.0))

(event `self.UpperBodyCollision.OnComponentBeginOverlap`
  (params (OverlappedComponent :type "PrimitiveComponent Object Reference") (OtherActor :type "Actor Object Reference") (OtherComp :type "PrimitiveComponent Object Reference") (OtherBodyIndex :type Integer) (bFromSweep :type Boolean) (SweepResult :type "HitResult Structure (by ref)"))
  (`KismetSystemLibrary.PrintText` (`|FormatText` "Fighter {Index} has been hit on the upper body !" (`self.FighterIndex`)) true true (struct :`R` 1.0 :`B` 0.237192 :`A` 1.0) 5.0))

(event `self.LowerBodyCollision.OnComponentBeginOverlap`
  (params (OverlappedComponent :type "PrimitiveComponent Object Reference") (OtherActor :type "Actor Object Reference") (OtherComp :type "PrimitiveComponent Object Reference") (OtherBodyIndex :type Integer) (bFromSweep :type Boolean) (SweepResult :type "HitResult Structure (by ref)"))
  (`KismetSystemLibrary.PrintText` (`|FormatText` "Fighter {Index} has been hit on the lower body !" (`self.FighterIndex`)) true true (struct :`R` 1.0 :`B` 0.237192 :`A` 1.0) 5.0))

(fn `ApplyTiltRotation`
  (params (RollValue :type "Float (double-precision)") (YawValue :type "Float (double-precision)"))
  (`SceneComponent.K2_SetRelativeRotation` (`self.Scene`) (`KismetMathLibrary.MakeRotator` RollValue 0.0 (`KismetMathLibrary.SelectFloat` 180.0 0.0 (== (`self.FighterIndex`) 1))) false false)
  (`SceneComponent.K2_SetRelativeRotation` (`self.FighterMesh`) (`KismetMathLibrary.MakeRotator` 90.0 0.0 YawValue) false false))

(fn `UserConstructionScript`)