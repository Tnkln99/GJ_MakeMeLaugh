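; BP_MainGameInstance tracks the scores of a two-player match, presumably as the Game Instance so they persist across level loads.
; Player1Win and Player2Win each add a point to their player's score, and ResetScores clears both.
; IsSomeBodyWon reports whether either player has reached the hardcoded three-point winning threshold.
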(fn `IsSomeBodyWon`
  (returns (Win :type Boolean))
  (return (or (>= (`self.Player1Score`) 3) (>= (`self.Player2Score`) 3))))

(fn `Player1Win`
  (`/Engine/EditorBlueprintResources/StandardMacros.IncrementInt` (`self.Player1Score`)))

(fn `Player2Win`
  (`/Engine/EditorBlueprintResources/StandardMacros.IncrementInt` (`self.Player2Score`)))

(fn `ResetScores`
  (set `self.Player1Score` 0)
  (set `self.Player2Score` 0))