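; BP_TestArm is a test actor for nudging a Sphere component by hand with debug keys.
; Four key press events add a fixed relative offset to the Sphere, with left and right moving it along local Y and up and down along local Z.
; BeginPlay, overlap, Tick and the construction script are empty, so key input is the only behavior.
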(event EventBeginPlay)

(event Collision|EventActorBeginOverlap
  (params (OtherActor :type Actor%20Object%20Reference)))

(event EventTick
  (params (DeltaSeconds :type Float%20%28single-precision%29)))

(event Input|KeyboardEvents|DebugKeyRight
  (params (Key :type Key%20Structure :default "None") (ActionValue :type Input%20Action%20Value%20Structure))
  (:Pressed
    (Transformation|AddRelativeLocation (Variables|Default|GetSphere) (Math|Vector|MakeVector 0.0 1e+01 0.0) false false)))

(event Input|KeyboardEvents|DebugKeyLeft
  (params (Key :type Key%20Structure :default "None") (ActionValue :type Input%20Action%20Value%20Structure))
  (:Pressed
    (Transformation|AddRelativeLocation (Variables|Default|GetSphere) (Math|Vector|MakeVector 0.0 -1e+01 0.0) false false)))

(event Input|KeyboardEvents|DebugKeyUp
  (params (Key :type Key%20Structure :default "None") (ActionValue :type Input%20Action%20Value%20Structure))
  (:Pressed
    (Transformation|AddRelativeLocation (Variables|Default|GetSphere) (Math|Vector|MakeVector 0.0 0.0 1e+01) false false)))

(event Input|KeyboardEvents|DebugKeyDown
  (params (Key :type Key%20Structure :default "None") (ActionValue :type Input%20Action%20Value%20Structure))
  (:Pressed
    (Transformation|AddRelativeLocation (Variables|Default|GetSphere) (Math|Vector|MakeVector 0.0 0.0 -1e+01) false false)))

(fn ConstructionScript)