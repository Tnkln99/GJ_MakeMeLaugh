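; BP_Controller turns Enhanced Input actions into roll and yaw tilting for the first BP_Fighter found in the level.
; BeginPlay caches that fighter and adds the fighters' input mapping context.
; Both actions feed TiltFighter, which accumulates clamped angles using a sensitivity that follows a curve over hold time.
; Roll sets the fighter's Scene world rotation, while yaw sets its mesh's relative rotation.
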(event `self.ReceiveBeginPlay`
  (`|ExecutionSequence`
    (:`then_0`
      (bind _outactors (`GameplayStatics.GetAllActorsOfClass` "/Game/Actors/BP_Fighter.BP_Fighter_C"))
      (for (_array_element _array_index) _outactors
        (if (== _array_index 0)
          (set `self.Fighter_1` _array_element))))
    (:`then_1`
      (`EnhancedInputSubsystemInterface.AddMappingContext` (subsystem `EnhancedInputLocalPlayerSubsystem`) "/Game/Inputs/IMC_Fighters.IMC_Fighters" 0 (struct))
      (`KismetSystemLibrary.PrintString` "Hello"))))

(event `EnhancedInput|/Game/Inputs/IA_TiltRollFighter1`
  (params (ActionValue :type "Float (double-precision)") (ElapsedSeconds :type "Float (double-precision)") (TriggeredSeconds :type "Float (double-precision)") (InputAction :type "InputAction Object Reference" :default "/Game/Inputs/IA_TiltRollFighter1.IA_TiltRollFighter1"))
  (:`Triggered`
    (`self.TiltFighter` "NewEnumerator0" ActionValue TriggeredSeconds (`self.Fighter_1`))))

(event `EnhancedInput|/Game/Inputs/IA_TiltYawFighter1`
  (params (ActionValue :type "Float (double-precision)") (ElapsedSeconds :type "Float (double-precision)") (TriggeredSeconds :type "Float (double-precision)") (InputAction :type "InputAction Object Reference" :default "/Game/Inputs/IA_TiltYawFighter1.IA_TiltYawFighter1"))
  (:`Triggered`
    (`self.TiltFighter` "NewEnumerator1" ActionValue TriggeredSeconds (`self.Fighter_1`))))

(fn `TiltFighter`
  (params (Tilt :type "/Game/Datas/E_Tilt Enum" :default "NewEnumerator0") (Value :type "Float (double-precision)") (Time :type "Float (double-precision)") (Fighter :type "/Game/Actors/BP_Fighter Object Reference"))
  (bind (_tiltsensitivity_min _tiltsensitivity_max) (break `FloatInterval` (`self.TiltSensitivity`)))
  (bind (_tiltrolllimits_min _tiltrolllimits_max) (break `FloatInterval` (`self.TiltRollLimits`)))
  (bind (_tiltyawlimits_min _tiltyawlimits_max) (break `FloatInterval` (`self.TiltYawLimits`)))
  (bind _returnvalue (* Value (`KismetMathLibrary.Lerp` _tiltsensitivity_min _tiltsensitivity_max (`CurveFloat.GetFloatValue` (`self.TiltCurve`) (/ Time (`self.TiltTime`))))))
  (switch `/Game/Datas/E_Tilt` Tilt
    (:`NewEnumerator0`
      (bind _output_get (set `self.TiltRoll` (`KismetMathLibrary.FClamp` (+ (`self.TiltRoll`) _returnvalue) _tiltrolllimits_min _tiltrolllimits_max)))
      (`SceneComponent.K2_SetWorldRotation` (`/Game/Actors/BP_Fighter.Scene` Fighter) (`KismetMathLibrary.MakeRotator` _output_get) false false))
    (:`NewEnumerator1`
      (bind _output_get_2 (set `self.TiltYaw` (`KismetMathLibrary.FClamp` (+ (`self.TiltYaw`) _returnvalue) _tiltyawlimits_min _tiltyawlimits_max)))
      (`SceneComponent.K2_SetRelativeRotation` (`/Game/Actors/BP_Fighter.FighterMesh` Fighter) (`KismetMathLibrary.MakeRotator` 90.0 0.0 _output_get_2) false false))))

(fn `UserConstructionScript`)