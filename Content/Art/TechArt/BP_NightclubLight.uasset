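; BP_NightclubLight is an animated nightclub spotlight that shifts color, intensity and position on a looping timeline.
; Construction sets the starting look and light function material, then creates a dynamic instance of it without assigning that instance back to the light.
; BeginPlay starts the timeline, whose alpha also drives the instance's Time parameter and offsets location from its current value each update.
; The timeline replays while Activatelight is true.
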(event `self.ReceiveBeginPlay`
  (`TimelineComponent.SetPlayRate` (`self.AnimLight`) (`self.PlayRateTimeLine`))
  (`self.light1`))

(event `light1`
  (bind _alpha (`self.Alpha`))
  (bind _spotlight (`self.SpotLight`))
  (bind _returnvalue (`SceneComponent.K2_GetComponentLocation` _spotlight))
  (bind _returnvalue_2 (/ (`self.BasePosition`) (10.0 10.0 10.0)))
  (bind (_direction _alpha_2) (`Timeline|AnimLight` :!via `PlayFromStart`)
    (:`Update`
      (bind _output_get (set `self.Alpha` _alpha_2))
      (`LightComponent.SetLightColor` (`self.SpotLight`) (`KismetMathLibrary.LinearColorLerp` (`self.ColorA`) (`self.ColorB`) _output_get) true)
      (`LightComponent.SetIntensity` (`self.SpotLight`) (`KismetMathLibrary.Lerp` (`self.Intensitylight A`) (`self.Itensitylight B`) _alpha))
      (`MaterialInstanceDynamic.SetScalarParameterValue` (`self.Sptolight1Mat`) "Time" (`KismetMathLibrary.Lerp` (`self.TimeMin`) (`self.TimeMax`) _alpha))
      (`SceneComponent.K2_SetWorldLocation` _spotlight (`KismetMathLibrary.VLerp` (+ _returnvalue _returnvalue_2) (- _returnvalue _returnvalue_2) (`self.Alpha`)) false false))
    (:`Finished`
      (if (`self.Activatelight`)
        (`self.light1`)))))

(fn `UserConstructionScript`
  (`LightComponent.SetLightFunctionMaterial` (`self.SpotLight`) (`self.Material`))
  (bind _returnvalue (`KismetMaterialLibrary.CreateDynamicMaterialInstance` (`LightComponent.LightFunctionMaterial` (`self.SpotLight`))))
  (set `self.Sptolight1Mat` _returnvalue)
  (`LightComponent.SetLightColor` (`self.SpotLight`) (`self.ColorA`) true)
  (`LightComponent.SetIntensity` (`self.SpotLight`) (`self.Intensitylight A`)))