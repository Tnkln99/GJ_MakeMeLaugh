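; BP_Tchoutchou is a train station environment actor, apparently an ambient train, that repeatedly travels along a straight path.
; On BeginPlay, the Aller event moves the Root component to TargetPosition over OverTime using MoveComponentTo.
; It then snaps Root back to a zero relative location without sweeping, waits a random few seconds and calls itself again, looping indefinitely.
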(event `Aller`
  (`KismetSystemLibrary.MoveComponentTo` (`self.Root`) (`self.TargetPosition`) (struct) false false (`self.Over Time`))
  (`SceneComponent.K2_SetRelativeLocation` (`self.Root`) (0.0 0.0 0.0) false false)
  (`KismetSystemLibrary.Delay` (`KismetMathLibrary.RandomFloatInRange` 5.0 10.0))
  (`self.Aller`))

(event `self.ReceiveBeginPlay`
  (`self.Aller`))

(fn `UserConstructionScript`)